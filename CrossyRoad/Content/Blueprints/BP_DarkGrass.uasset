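; Grass lane actor for a lane-hopping game, with tree borders, side blockers and randomly placed obstacles.
; On BeginPlay it randomizes the border tree mesh and, if the game has started, scatters tree or rock BP_Obstacle actors between two markers.
; Trigger zones notify BP_MyCharacter to block sideways moves, score once or spawn the eagle.
; A destroy zone removes the lane and its tracked obstacles when the player overlaps it.
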(event OnComponentBeginOverlap(LeftSideBlock)
  (params (OverlappedComponent :type Primitive%20Component%20Object%20Reference) (OtherActor :type Actor%20Object%20Reference) (OtherComp :type Primitive%20Component%20Object%20Reference) (OtherBodyIndex :type Integer) (bFromSweep :type Boolean) (SweepResult :type Hit%20Result%20Structure%20%28by%20ref%29))
  (bind _asbp_my_character (Utilities|Casting|CastToBP_MyCharacter OtherActor))
  (Default|LeftBlock _asbp_my_character))

(event OnComponentBeginOverlap(RightSideBlock)
  (params (OverlappedComponent :type Primitive%20Component%20Object%20Reference) (OtherActor :type Actor%20Object%20Reference) (OtherComp :type Primitive%20Component%20Object%20Reference) (OtherBodyIndex :type Integer) (bFromSweep :type Boolean) (SweepResult :type Hit%20Result%20Structure%20%28by%20ref%29))
  (bind _asbp_my_character (Utilities|Casting|CastToBP_MyCharacter OtherActor))
  (Default|RightBlock _asbp_my_character))

(event OnComponentBeginOverlap(LaneDestroyZone)
  (params (OverlappedComponent :type Primitive%20Component%20Object%20Reference) (OtherActor :type Actor%20Object%20Reference) (OtherComp :type Primitive%20Component%20Object%20Reference) (OtherBodyIndex :type Integer) (bFromSweep :type Boolean) (SweepResult :type Hit%20Result%20Structure%20%28by%20ref%29))
  (bind _obstacle_array (Variables|Default|GetObstacle_Array))
  ;[1 1 1] Handle Destroying Lanes
  (Utilities|Casting|CastToBP_MyCharacter OtherActor)
  (Actor|DestroyActor)
  ;[1 1 1] Hande destroying all BP_Vehicle meshes within lane
  (for (_array_element _array_index) _obstacle_array
    (Actor|DestroyActor _array_element)
    (Utilities|Array|SetArrayElem (Variables|Default|GetObstacle_Array) _array_index 0))
  (Utilities|Array|Clear _obstacle_array))

(event OnComponentHit(EagleKillZone)
  (params (HitComponent :type Primitive%20Component%20Object%20Reference) (OtherActor :type Actor%20Object%20Reference) (OtherComp :type Primitive%20Component%20Object%20Reference) (NormalImpulse :type Vector :default "0, 0, 0") (Hit :type Hit%20Result%20Structure%20%28by%20ref%29))
  (Utilities|FlowControl|DoOnce false
    (:Completed
      (bind _asbp_my_character (Utilities|Casting|CastToBP_MyCharacter OtherActor))
      (Default|SpawnEagle _asbp_my_character))))

(event OnComponentBeginOverlap(ScoringZone)
  (params (OverlappedComponent :type Primitive%20Component%20Object%20Reference) (OtherActor :type Actor%20Object%20Reference) (OtherComp :type Primitive%20Component%20Object%20Reference) (OtherBodyIndex :type Integer) (bFromSweep :type Boolean) (SweepResult :type Hit%20Result%20Structure%20%28by%20ref%29))
  (bind _asbp_my_character (Utilities|Casting|CastToBP_MyCharacter OtherActor))
  (Utilities|FlowControl|DoOnce false
    (:Completed
      (Default|UpdateScore _asbp_my_character))))

(event EventBeginPlay
  ;[1 1 1] Set Bounding Trees to random type
  (bind _output_get (Variables|Default|SetWorld_Bound_Tree_Type (Math|Random|RandomIntegerinRange 0 2)))
  (Components|StaticMesh|SetStaticMesh (Variables|Default|Gettree) (Utilities|Select :Index _output_get :Option%200 "/Game/Meshes/Obstacles/LargeTree.LargeTree" :Option%201 "/Game/Meshes/Obstacles/MediumTree.MediumTree" :Option%202 "/Game/Meshes/Obstacles/SmallTree.SmallTree"))
  (Components|StaticMesh|SetStaticMesh (Variables|Default|Gettree1) (Utilities|Select :Index _output_get :Option%200 "/Game/Meshes/Obstacles/LargeTree.LargeTree" :Option%201 "/Game/Meshes/Obstacles/MediumTree.MediumTree" :Option%202 "/Game/Meshes/Obstacles/SmallTree.SmallTree"))
  (Components|StaticMesh|SetStaticMesh (Variables|Default|Gettree2) (Utilities|Select :Index _output_get :Option%200 "/Game/Meshes/Obstacles/LargeTree.LargeTree" :Option%201 "/Game/Meshes/Obstacles/MediumTree.MediumTree" :Option%202 "/Game/Meshes/Obstacles/SmallTree.SmallTree"))
  (Components|StaticMesh|SetStaticMesh (Variables|Default|Gettree3) (Utilities|Select :Index _output_get :Option%200 "/Game/Meshes/Obstacles/LargeTree.LargeTree" :Option%201 "/Game/Meshes/Obstacles/MediumTree.MediumTree" :Option%202 "/Game/Meshes/Obstacles/SmallTree.SmallTree"))
  (Variables|Default|SetLane_Tree_Type (Math|Random|RandomIntegerinRange 0 3))
  (Variables|Default|SetRandom_Start (Transformation|GetWorldLocation (Variables|Default|GetRandomStart)))
  (Variables|Default|SetRandom_End (Transformation|GetWorldLocation (Variables|Default|GetRandomEnd)))
  (bind _asbp_my_character (Utilities|Casting|CastToBP_MyCharacter (Game|GetPlayerCharacter 0)))
  (if (Variables|/Game/Blueprints/BP_MyCharacter.BP_MyCharacter_C|GetGame_Start _asbp_my_character)
    (for _index (range 0 (Math|Float|Truncate (/ (Math|Vector|Distance(Vector) (Variables|Default|GetRandom_Start) (Variables|Default|GetRandom_End)) 9e+01)))
      (if (> (Math|Random|RandomFloat) 0.8)
        (if (> (Math|Random|RandomFloat) 0.5)
          (CallFunction|SpawnObstacle (Math|Vector|MakeVector (.x (+ (Math|Vector|MakeVector (.x (Variables|Default|GetRandom_Start)) 0.0 0.0) (* _index 80))) (.y (Variables|Default|GetRandom_Start)) (.z (Variables|Default|GetRandom_Start)))))))))

(fn ConstructionScript)

(fn SpawnObstacle
  (params (Location :type Vector))
  ;[1 1 1] Spawn a Vehicle in Lane Based on Direction
  (if (> (Math|Random|RandomFloat) 0.5)
    (bind _returnvalue (Game|SpawnActorfromClass "/Game/Blueprints/BP_Obstacle.BP_Obstacle_C" (Math|Transform|MakeTransform Location "0, 0, 0" "1,1,1") "Undefined" 0 0))
    (bind _output_get (Variables|Default|SetObstacle _returnvalue))
    (Utilities|Array|Add (Variables|Default|GetObstacle_Array) _output_get)
    (Components|StaticMesh|SetStaticMesh (Variables|/Game/Blueprints/BP_Obstacle.BP_Obstacle_C|GetStaticMesh (Variables|Default|GetObstacle)) (Utilities|Select :Index (Variables|Default|GetLane_Tree_Type) :Option%200 "/Game/Meshes/Obstacles/SmallTree.SmallTree" :Option%201 "/Game/Meshes/Obstacles/MediumTree.MediumTree" :Option%202 "/Game/Meshes/Obstacles/palm_tree.palm_tree" :Option%203 "/Game/Meshes/Obstacles/italian_cypress.italian_cypress"))
    (else
      (bind _returnvalue_2 (Game|SpawnActorfromClass "/Game/Blueprints/BP_Obstacle.BP_Obstacle_C" (Math|Transform|MakeTransform Location "0, 0, 0" "1,1,1") "Undefined" 0 0))
      (bind _output_get_2 (Variables|Default|SetObstacle _returnvalue_2))
      (Utilities|Array|Add (Variables|Default|GetObstacle_Array) _output_get_2)
      (Components|StaticMesh|SetStaticMesh (Variables|/Game/Blueprints/BP_Obstacle.BP_Obstacle_C|GetStaticMesh (Variables|Default|GetObstacle)) (Utilities|Select :Index (Math|Random|RandomIntegerinRange 0 1) :Option%200 "/Game/Meshes/Obstacles/centerrock1.centerrock1" :Option%201 "/Game/Meshes/Obstacles/centerrock2.centerrock2")))))