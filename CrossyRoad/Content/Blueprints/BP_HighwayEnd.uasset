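; BP_HighwayEnd is a highway lane actor for a chicken road-crossing game, spawning traffic at a random direction and speed chosen on BeginPlay.
; A frame-based Tick countdown spawns BP_Vehicles with random meshes at either end and tracks them in CarArray.
; Kill zones remove passing vehicles, and LaneDestroyZone destroys the lane and its cars when the player overlaps it.
; Other colliders block sideways movement, update score and trigger the eagle on the player.
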(event OnComponentBeginOverlap(LeftSideBlock)
  (params (OverlappedComponent :type Primitive%20Component%20Object%20Reference) (OtherActor :type Actor%20Object%20Reference) (OtherComp :type Primitive%20Component%20Object%20Reference) (OtherBodyIndex :type Integer) (bFromSweep :type Boolean) (SweepResult :type Hit%20Result%20Structure%20%28by%20ref%29))
  ;[1 1 1] Handle Chicken running into bounds
  (bind _asbp_my_character (Utilities|Casting|CastToBP_MyCharacter OtherActor))
  (Default|LeftBlock _asbp_my_character))

(event OnComponentBeginOverlap(RightSideBlock)
  (params (OverlappedComponent :type Primitive%20Component%20Object%20Reference) (OtherActor :type Actor%20Object%20Reference) (OtherComp :type Primitive%20Component%20Object%20Reference) (OtherBodyIndex :type Integer) (bFromSweep :type Boolean) (SweepResult :type Hit%20Result%20Structure%20%28by%20ref%29))
  ;[1 1 1] Handle Chicken running into bounds
  (bind _asbp_my_character (Utilities|Casting|CastToBP_MyCharacter OtherActor))
  (Default|RightBlock _asbp_my_character))

(event OnComponentBeginOverlap(Destroy_Right)
  (params (OverlappedComponent :type Primitive%20Component%20Object%20Reference) (OtherActor :type Actor%20Object%20Reference) (OtherComp :type Primitive%20Component%20Object%20Reference) (OtherBodyIndex :type Integer) (bFromSweep :type Boolean) (SweepResult :type Hit%20Result%20Structure%20%28by%20ref%29))
  ;[1 1 1] Destroy the Vehicles as they cross the killzones
  (bind _asbp_vehicle (Utilities|Casting|CastToBP_Vehicle OtherActor))
  (Actor|DestroyActor _asbp_vehicle)
  (Utilities|Array|RemoveItem (Variables|Default|GetCar_Array) _asbp_vehicle))

(event OnComponentBeginOverlap(LaneDestroyZone)
  (params (OverlappedComponent :type Primitive%20Component%20Object%20Reference) (OtherActor :type Actor%20Object%20Reference) (OtherComp :type Primitive%20Component%20Object%20Reference) (OtherBodyIndex :type Integer) (bFromSweep :type Boolean) (SweepResult :type Hit%20Result%20Structure%20%28by%20ref%29))
  (bind _car_array (Variables|Default|GetCar_Array))
  ;[1 1 1] Handle destroying lanes
  (Utilities|Casting|CastToBP_MyCharacter OtherActor)
  (Actor|DestroyActor)
  ;[1 1 1] Hande destroying all BP_Vehicle meshes within lane
  (for (_array_element _array_index) _car_array
    (Actor|DestroyActor _array_element)
    (Utilities|Array|SetArrayElem (Variables|Default|GetCar_Array) _array_index 0))
  (Utilities|Array|Clear _car_array))

(event OnComponentBeginOverlap(Destroy_Left)
  (params (OverlappedComponent :type Primitive%20Component%20Object%20Reference) (OtherActor :type Actor%20Object%20Reference) (OtherComp :type Primitive%20Component%20Object%20Reference) (OtherBodyIndex :type Integer) (bFromSweep :type Boolean) (SweepResult :type Hit%20Result%20Structure%20%28by%20ref%29))
  ;[1 1 1] Destroy the Vehicles as they cross the killzones
  (bind _asbp_vehicle (Utilities|Casting|CastToBP_Vehicle OtherActor))
  (Actor|DestroyActor _asbp_vehicle)
  (Utilities|Array|RemoveItem (Variables|Default|GetCar_Array) _asbp_vehicle))

(event OnComponentHit(EagleKillZone)
  (params (HitComponent :type Primitive%20Component%20Object%20Reference) (OtherActor :type Actor%20Object%20Reference) (OtherComp :type Primitive%20Component%20Object%20Reference) (NormalImpulse :type Vector :default "0, 0, 0") (Hit :type Hit%20Result%20Structure%20%28by%20ref%29))
  (Utilities|FlowControl|DoOnce false
    (:Completed
      (bind _asbp_my_character (Utilities|Casting|CastToBP_MyCharacter OtherActor))
      (Default|SpawnEagle _asbp_my_character))))

(event OnComponentBeginOverlap(ScoringZone)
  (params (OverlappedComponent :type Primitive%20Component%20Object%20Reference) (OtherActor :type Actor%20Object%20Reference) (OtherComp :type Primitive%20Component%20Object%20Reference) (OtherBodyIndex :type Integer) (bFromSweep :type Boolean) (SweepResult :type Hit%20Result%20Structure%20%28by%20ref%29))
  (bind _asbp_my_character (Utilities|Casting|CastToBP_MyCharacter OtherActor))
  (Utilities|FlowControl|DoOnce false
    (:Completed
      (Default|UpdateScore _asbp_my_character))))

(event EventBeginPlay
  (bind _max_lane_speed (Variables|Default|GetMax_Lane_Speed))
  (bind _min_lane_speed (Variables|Default|GetMin_Lane_Speed))
  ;[1 1 1] Set Initial Spawning Variables of the Lane (Spawn Times, Vehicle Direction, and Vehicle Speed)
  (Variables|Default|SetDirection (Math|Random|RandomBool))
  (Variables|Default|SetSpawn_Time (* (Math|Random|RandomIntegerinRange (Variables|Default|GetMin_Spawn_Time) (Variables|Default|GetMax_Spawn_Time)) 10))
  (if (Variables|Default|GetDirection)
    (Variables|Default|SetLane_Speed (* (Math|Random|RandomFloatinRange _min_lane_speed _max_lane_speed) 5e+01))
    (else
      (Variables|Default|SetLane_Speed (* (Math|Random|RandomFloatinRange _min_lane_speed _max_lane_speed) -5e+01)))))

(event EventTick
  (params (DeltaSeconds :type Float%20%28single-precision%29))
  ;[1 1 1] Handle Spawning the Vehicles in Lane
  ;;[1 1 1] Decrement Spawn Time and Spawn Vehicle if equal to 0
  (Math|Integer|DecrementInt (Variables|Default|GetSpawn_Time)
    (:%20%20
      (if (== (Variables|Default|GetSpawn_Time) 0)
        (CallFunction|SpawnVehicle)
        (Variables|/Game/Blueprints/BP_Vehicle.BP_Vehicle_C|SetSet_Speed (Variables|Default|GetVehicle) (Variables|Default|GetLane_Speed))
        (Variables|Default|SetSpawn_Time (* (Math|Random|RandomIntegerinRange (Variables|Default|GetMin_Spawn_Time) (Variables|Default|GetMax_Spawn_Time)) 10))
        (Components|StaticMesh|SetStaticMesh (Variables|/Game/Blueprints/BP_Vehicle.BP_Vehicle_C|GetStaticMesh (Variables|Default|GetVehicle)) (Utilities|Select :Index (Math|Random|RandomIntegerinRange 0 8) :Option%200 "/Game/Meshes/Cars/darkgreen_blue_car_Untitled_001.darkgreen_blue_car_Untitled_001" :Option%201 "/Game/Meshes/Cars/darkgreen_car_Untitled_002.darkgreen_car_Untitled_002" :Option%202 "/Game/Meshes/Cars/darkgreen_orange_car.darkgreen_orange_car" :Option%203 "/Game/Meshes/Cars/short_blue_car.short_blue_car" :Option%204 "/Game/Meshes/Cars/short_red_car.short_red_car" :Option%205 "/Game/Meshes/Cars/FedEx_Truck.FedEx_Truck" :Option%206 "/Game/Meshes/Cars/taxi.taxi" :Option%207 "/Game/Meshes/Cars/police.police" :Option%208 "/Game/Meshes/Cars/ups.ups" :Option%209 0))))))

(fn ConstructionScript)

(fn SpawnVehicle
  ;[1 1 1] Spawn a Vehicle in Lane Based on Direction
  (if (Variables|Default|GetDirection)
    (bind _output_get (Variables|Default|SetStart (Transformation|GetWorldLocation (Variables|Default|GetLeft_Spawn))))
    (bind _returnvalue (Game|SpawnActorfromClass "/Game/Blueprints/BP_Vehicle.BP_Vehicle_C" (Math|Transform|MakeTransform _output_get "0, 0, 0" "1,1,1") "Undefined" 0 0))
    (bind _output_get_2 (Variables|Default|SetVehicle _returnvalue))
    (Utilities|Array|Add (Variables|Default|GetCar_Array) _output_get_2)
    (else
      (bind _output_get_3 (Variables|Default|SetStart (Transformation|GetWorldLocation (Variables|Default|GetRight_Spawn))))
      (bind _returnvalue_2 (Game|SpawnActorfromClass "/Game/Blueprints/BP_Vehicle.BP_Vehicle_C" (Math|Transform|MakeTransform _output_get_3 "0.000000,180.000000, 0" "1,1,1") "Undefined" 0 0))
      (bind _output_get_4 (Variables|Default|SetVehicle _returnvalue_2))
      (Utilities|Array|Add (Variables|Default|GetCar_Array) _output_get_4))))