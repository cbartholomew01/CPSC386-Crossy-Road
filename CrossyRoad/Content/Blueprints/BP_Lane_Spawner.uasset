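; Procedural lane spawner that builds endless terrain ahead of the chicken player from grass, river, railroad and highway lanes.
; On BeginPlay it lays a random count of lanes along Y (fixed until game start), opening with grass and choosing the rest randomly.
; Grass and highway flags on BP_MyCharacter help sequence lanes across spawners.
; An early trigger zone spawns the next spawner past the last lane when the player overlaps it.
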(event Custom|OnActorBeginOverlap_Event_1
  (params (OverlappedActor :type Actor%20Object%20Reference) (OtherActor :type Actor%20Object%20Reference))
  (bind _staticmesh (Variables|Default|GetStaticMesh))
  (bind _returnvalue (Transformation|GetWorldLocation _staticmesh))
  ;[1 1 1] Infinite Lane Spawner
  ;;[1 1 1] Spawn Trigger Zone and Check for Overlap once index reaches 3
  (Utilities|Casting|CastToBP_MyCharacter OtherActor)
  ;;[1 1 1] Once collision detected spawn lanes ahead of last index from prevous BP_Lane Spawner
  (Utilities|FlowControl|DoOnce false
    (:Completed
      (bind _output_get (Variables|Default|SetSpawnLocation (Math|Vector|MakeVector (.x _returnvalue) (+ (.y _returnvalue) (Math|Conversions|ToFloat(Integer) (+ (* (Variables|Default|GetLane_Index) 100) 100))) (.z _returnvalue))))
      (Game|SpawnActorfromClass "BP_Lane_Spawner_C" (Math|Transform|MakeTransform _output_get "0, 0, 0" "1,1,1") "Undefined" 0 0))))

(event EventBeginPlay
  (bind _staticmesh (Variables|Default|GetStaticMesh))
  (bind _returnvalue (Transformation|GetWorldLocation _staticmesh))
  ;[1 1 1] At Spawn get variables from BP_MyCharacter to avoid double light grass spawns/incorrect highway spawns
  (bind _outactors (Actor|GetAllActorsOfClass "/Game/Blueprints/BP_MyCharacter.BP_MyCharacter_C"))
  (bind _output_get (Variables|Default|SetChicken (Utilities|Array|Get(acopy) _outactors)))
  (Variables|Default|SetGrass_Switch (Variables|/Game/Blueprints/BP_MyCharacter.BP_MyCharacter_C|GetGrass_Switch _output_get))
  (Variables|Default|SetHighway_Marked (Variables|/Game/Blueprints/BP_MyCharacter.BP_MyCharacter_C|GetHighway_Marked _output_get))
  ;[1 1 1] Generate first lane type at spawn and # of lanes
  (Variables|Default|SetNextLane (Math|Random|RandomIntegerinRange 0 (Variables|Default|GetLane_Types)))
  (Variables|Default|SetLane_Index (Math|Random|RandomIntegerinRange (Variables|Default|GetMin_Lanes) (Variables|Default|GetMax_Lanes)))
  (bind _asbp_my_character (Utilities|Casting|CastToBP_MyCharacter (Game|GetPlayerCharacter 0)))
  (if (Variables|/Game/Blueprints/BP_MyCharacter.BP_MyCharacter_C|GetGame_Start _asbp_my_character)
    _
    (else
      (Variables|Default|SetLane_Index 10)))
  (for _index (range 0 (Variables|Default|GetLane_Index))
    ;[1 1 1] Set proper spacing between lanes depending on index
    (Variables|Default|SetSpawnLocation (Math|Vector|MakeVector (.x _returnvalue) (+ (Math|Conversions|ToFloat(Integer) (* _index 100)) (.y _returnvalue)) (.z _returnvalue)))
    (if (Math|Integer|InRange(Integer) _index 0 2)
      ;[1 1 1] Alternating Grass Spawner
      (if (Variables|Default|GetGrass_Switch) :!label _label
        (Game|SpawnActorfromClass "/Game/Blueprints/BP_LightGrass.BP_LightGrass_C" (Math|Transform|MakeTransform (Variables|Default|GetSpawnLocation) "0, 0, 0" "1,1,1") "Undefined" 0 0)
        (Variables|Default|SetGrass_Switch false)
        (Variables|Default|SetNextLane (Math|Random|RandomIntegerinRange 0 (Variables|Default|GetLane_Types)))
        (else
          (Game|SpawnActorfromClass "/Game/Blueprints/BP_DarkGrass.BP_DarkGrass_C" (Math|Transform|MakeTransform (Variables|Default|GetSpawnLocation) "0, 0, 0" "1,1,1") "Undefined" 0 0)
          (Variables|Default|SetGrass_Switch true)
          (Variables|Default|SetNextLane (Math|Random|RandomIntegerinRange 0 (Variables|Default|GetLane_Types)))))
      ;[1 1 1] After grass spawned update variable in BP_MyCharacter
      (bind _outactors_2 (Actor|GetAllActorsOfClass "/Game/Blueprints/BP_MyCharacter.BP_MyCharacter_C"))
      (Variables|/Game/Blueprints/BP_MyCharacter.BP_MyCharacter_C|SetGrass_Switch (Utilities|Array|Get(acopy) _outactors_2) (Variables|Default|GetGrass_Switch))
      (elif (Math|Integer|InRange(Integer) _index 4 (Variables|Default|GetLane_Index))
        ;[1 1 1] Select whether or not to spawn a marked highway lane
        (if (Math|Boolean|NANDBoolean (Variables|Default|GetHighway_Marked) (!= (Variables|Default|GetNextLane) 4)) :!label _label_2
          ;[1 1 1] Avoid last lane spawned being a highway
          (if (== _index (Variables|Default|GetLane_Index))
            (Variables|Default|SetNextLane (Math|Random|RandomIntegerinRange 0 3)))
          (switch int (Variables|Default|GetNextLane)
            (:0
              (goto _label))
            (:1
              (goto _label))
            (:2
              ;[1 1 1] River Spawner
              (Game|SpawnActorfromClass "/Game/Blueprints/BP_River.BP_River_C" (Math|Transform|MakeTransform (Variables|Default|GetSpawnLocation) "0, 0, 0" "1,1,1") "Undefined" 0 0)
              (Variables|Default|SetNextLane (Math|Random|RandomIntegerinRange 0 (Variables|Default|GetLane_Types))))
            (:3
              ;[1 1 1] RailRoad Spawner
              (Game|SpawnActorfromClass "/Game/Blueprints/BP_RailRoad.BP_RailRoad_C" (Math|Transform|MakeTransform (Variables|Default|GetSpawnLocation) "0, 0, 0" "1,1,1") "Undefined" 0 0)
              (Variables|Default|SetNextLane (Math|Random|RandomIntegerinRange 0 (Variables|Default|GetLane_Types))))
            (:4
              ;[1 1 1] Highway Spawner (Single + Multi Lanes)
              (Game|SpawnActorfromClass "/Game/Blueprints/BP_HighwayMarked.BP_HighwayMarked_C" (Math|Transform|MakeTransform (Variables|Default|GetSpawnLocation) "0, 0, 0" "1,1,1") "Undefined" 0 0)
              (Variables|Default|SetNextLane (Math|Random|RandomIntegerinRange 0 4))
              (Variables|Default|SetHighway_Marked true)
              ;[1 1 1] After highway spawned update variable in BP_MyCharacter
              (bind _outactors_3 (Actor|GetAllActorsOfClass "/Game/Blueprints/BP_MyCharacter.BP_MyCharacter_C" :!label _label_3))
              (Variables|/Game/Blueprints/BP_MyCharacter.BP_MyCharacter_C|SetHighway_Marked (Utilities|Array|Get(acopy) _outactors_3) false))
            (:5
              (Game|SpawnActorfromClass "/Game/Blueprints/BP_HighwayEnd.BP_HighwayEnd_C" (Math|Transform|MakeTransform (Variables|Default|GetSpawnLocation) "0, 0, 0" "1,1,1") "Undefined" 0 0 :!label _label_4)
              (Variables|Default|SetNextLane (Math|Random|RandomIntegerinRange 0 3))
              (Variables|Default|SetHighway_Marked false)
              (goto _label_3)))
          (else
            (goto _label_4)))
        (else
          ;[1 1 1] Infinite Lane Spawner
          ;;[1 1 1] Spawn Trigger Zone and Check for Overlap once index reaches 3
          (if (== _index 3)
            (bind _returnvalue_2 (Game|SpawnActorfromClass "/Game/Blueprints/BP_TriggerZone.BP_TriggerZone_C" (Math|Transform|MakeTransform (Variables|Default|GetSpawnLocation) "0, 0, 0" "1,1,1") "Undefined" 0 0))
            (EventDispatchers|AssignOnActorBeginOverlap _returnvalue_2 (delegate Custom|OnActorBeginOverlap_Event_1))
            (goto _label_2)))))))

(fn ConstructionScript)