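; Player chicken character for a Crossy Road-style hopper, handling movement, scoring, deaths and the HUD.
; Axis input launches grid-like hops, gated by CanMove and an InAir flag cleared on landing.
; Hazard events for cars and river disable movement, play effects and show the game-over widget, while score events count coins and save new high scores.
; A per-tick idle countdown, reset on landing, spawns an eagle and freezes the player once scoring has begun.
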(event Custom|Jumped%20Into%20Car
  (bind _returnvalue (Transformation|GetActorLocation))
  ;[1 1 1] Handle Game Over Case
  (if (Variables|Default|GetCan_Move)
    (Utilities|FlowControl|DoOnce false
      (:Completed
        (Character|LaunchCharacter "-1.000000,-1.000000, 0" true true)
        (Transformation|SetWorldScale3D (Variables|Default|GetChicken) "0.300000,0.030000,0.300000")
        (Variables|Default|SetCan_Move false)
        (Audio|PlaySoundatLocation "/Game/Audio/Hit_Cue.Hit_Cue" _returnvalue "0, 0, 0" 1.0 1.0 0.0 0 0 0)
        (Audio|PlaySoundatLocation "/Game/Audio/shriek_Cue.shriek_Cue" _returnvalue "0, 0, 0" 1.0 1.0 0.0 0 0 0)
        (bind _returnvalue_2 (UserInterface|CreateWidget "/Game/UI/WBP_GameOVer.WBP_GameOver_C"))
        (UserInterface|Viewport|AddtoViewport _returnvalue_2 0)
        (Variables|/Script/Engine.PlayerController|SetbShowMouseCursor (Game|GetPlayerController 0) true)
        (Variables|Default|SetGame_Start false)))))

(event Custom|Run%20Over
  (bind _returnvalue (Transformation|GetActorLocation))
  ;[1 1 1] Handle Game Over Case
  (if (Variables|Default|GetCan_Move)
    (Utilities|FlowControl|DoOnce false
      (:Completed
        (Character|LaunchCharacter "0.000000,-1.000000, 0" true true)
        (Transformation|AddWorldOffset (Variables|Default|GetChicken) "0, 0,-60.000000" true false)
        (Transformation|SetWorldScale3D (Variables|Default|GetChicken) "0.300000,0.300000,0.030000")
        (Variables|Default|SetCan_Move false)
        (Audio|PlaySoundatLocation "/Game/Audio/Hit_Cue.Hit_Cue" _returnvalue "0, 0, 0" 1.0 1.0 0.0 0 0 0)
        (Audio|PlaySoundatLocation "/Game/Audio/shriek_Cue.shriek_Cue" _returnvalue "0, 0, 0" 1.0 1.0 0.0 0 0 0)
        (bind _returnvalue_2 (UserInterface|CreateWidget "/Game/UI/WBP_GameOVer.WBP_GameOver_C"))
        (UserInterface|Viewport|AddtoViewport _returnvalue_2 0)
        (Variables|/Script/Engine.PlayerController|SetbShowMouseCursor (Game|GetPlayerController 0) true)
        (Variables|Default|SetGame_Start false)))))

(event Custom|Left%20Block
  ;[1 1 1] Handle running into world bounds
  (Character|LaunchCharacter "200.000000,0.000000,0.000000" true true))

(event Custom|Right%20Block
  ;[1 1 1] Handle running into world bounds
  (Character|LaunchCharacter "-200.000000,0.000000, 0" true true))

(event Custom|RiverRunoff
  ;[1 1 1] Handle Game Over Case
  (Variables|Default|SetCan_Move false)
  (Audio|PlaySoundatLocation "/Game/Audio/shriek_Cue.shriek_Cue" (Transformation|GetActorLocation) "0, 0, 0" 1.0 1.0 0.0 0 0 0)
  (bind _returnvalue (UserInterface|CreateWidget "/Game/UI/WBP_GameOVer.WBP_GameOver_C"))
  (UserInterface|Viewport|AddtoViewport _returnvalue 0)
  (Variables|/Script/Engine.PlayerController|SetbShowMouseCursor (Game|GetPlayerController 0) true)
  (Variables|Default|SetGame_Start false))

(event Custom|Update_Score
  (bind _result (Math|Float|IncrementFloat (Variables|Default|GetScore))
    (:%20%20
      (bind _output_get (Variables|Default|SetScore _result))
      (if (>= _output_get (Variables|Default|GetHigh_Score))
        (Variables|Default|SetHigh_Score _output_get)
        (bind _returnvalue (SaveGame|DoesSaveGameExist (Variables|Default|GetHigh_Score_Slot)))
        (if _returnvalue
          (bind _returnvalue_2 (SaveGame|LoadGamefromSlot (Variables|Default|GetHigh_Score_Slot)))
          (bind _output_get_2 (Variables|Default|SetSaveGameReference _returnvalue_2))
          (bind _asbp_save_game (Utilities|Casting|CastToBP_SaveGame _output_get_2))
          (Variables|/Game/Blueprints/BP_SaveGame.BP_SaveGame_C|SetHigh_Score _asbp_save_game (Math|Float|Truncate (Variables|Default|GetHigh_Score)))
          (else
            (bind _returnvalue_3 (SaveGame|CreateSaveGameObject "/Game/Blueprints/BP_SaveGame.BP_SaveGame_C"))
            (bind _output_get_3 (Variables|Default|SetSaveGameReference _returnvalue_3))
            (bind _asbp_save_game_2 (Utilities|Casting|CastToBP_SaveGame _output_get_3))
            (Variables|/Game/Blueprints/BP_SaveGame.BP_SaveGame_C|SetHigh_Score _asbp_save_game_2 (Math|Float|Truncate (Variables|Default|GetHigh_Score)))))
        (SaveGame|SaveGametoSlot (Variables|Default|GetSaveGameReference) (Variables|Default|GetHigh_Score_Slot))))))

(event Custom|Update_Coins
  (bind _result (Math|Float|IncrementFloat (Variables|Default|GetCoins_Collected))
    (:%20%20
      (Variables|Default|SetCoins_Collected _result))))

(event Custom|Fallen%20in%20River
  (bind _returnvalue (Transformation|GetActorLocation))
  ;[1 1 1] Handle Game Over Case
  (if (Variables|Default|GetCan_Move)
    (Components|StaticMesh|SetStaticMesh (Variables|Default|GetWater_Explosion) "/Game/Meshes/water_explosion.water_explosion")
    (Audio|PlaySoundatLocation "/Game/Audio/splash_Cue.splash_Cue" _returnvalue "0, 0, 0" 1.0 1.0 0.0 0 0 0)
    (Audio|PlaySoundatLocation "/Game/Audio/shriek_Cue.shriek_Cue" _returnvalue "0, 0, 0" 1.0 1.0 0.0 0 0 0)
    (bind _newtrack_0 (Timeline|Timeline_0 Play)
      (:Update
        (Transformation|AddWorldOffset (Variables|Default|GetWater_Explosion) (Math|Vector|MakeVector 0.0 0.0 (* _newtrack_0 15.0)) true false))
      (:Finished
        (Transformation|SetWorldScale3D (Variables|Default|GetChicken) "0.300000,0.300000,0.030000")
        (Variables|Default|SetCan_Move false)
        (bind _returnvalue_2 (UserInterface|CreateWidget "/Game/UI/WBP_GameOVer.WBP_GameOver_C"))
        (UserInterface|Viewport|AddtoViewport _returnvalue_2 0)
        (Variables|/Script/Engine.PlayerController|SetbShowMouseCursor (Game|GetPlayerController 0) true)
        (Variables|Default|SetGame_Start false)))))

(event Custom|Spawn_Eagle
  (bind _returnvalue (Transformation|GetActorLocation))
  (bind _returnvalue_2 (Game|SpawnActorfromClass "/Game/Blueprints/BP_Eagle.BP_Eagle_C" (Math|Transform|MakeTransform (Math|Vector|MakeVector (.x _returnvalue) (+ (.y _returnvalue) 1e+03) (.z _returnvalue)) "0, 0, 0" "1,1,1") "Undefined" 0 0))
  (Variables|Default|SetCan_Move false)
  (Default|SpawnEagle _returnvalue_2)
  (Audio|PlaySoundatLocation "/Game/Audio/Eagle.Eagle" (Transformation|GetActorLocation) "0, 0, 0" 1.0 1.0 0.0 0 0 0))

(event EventBeginPlay
  (bind _returnvalue (SaveGame|DoesSaveGameExist "High_Score_Slot"))
  (if _returnvalue
    (bind _returnvalue_2 (SaveGame|LoadGamefromSlot (Variables|Default|GetHigh_Score_Slot)))
    (bind _output_get (Variables|Default|SetSaveGameReference _returnvalue_2))
    (bind _asbp_save_game (Utilities|Casting|CastToBP_SaveGame _output_get))
    (Variables|Default|SetHigh_Score (Math|Conversions|ToFloat(Integer) (Variables|/Game/Blueprints/BP_SaveGame.BP_SaveGame_C|GetHigh_Score _asbp_save_game))))
  (bind _returnvalue_3 (UserInterface|CreateWidget "/Game/UI/WBP_HUD.WBP_HUD_C"))
  (UserInterface|Viewport|AddtoViewport _returnvalue_3 0)
  (Variables|Default|SetGame_Start false))

(event EventOnLanded
  (params (Hit :type Hit%20Result%20Structure%20%28by%20ref%29))
  ;[1 1 1] Chicken Movement
  (Variables|Default|SetInAir false)
  (Variables|Default|SetEagle_Spawn 150))

(event EventTick
  (params (DeltaSeconds :type Float%20%28single-precision%29))
  (if (and (> (Variables|Default|GetScore) 0.0) (Variables|Default|GetCan_Move))
    (bind _result (Math|Integer|DecrementInt (Variables|Default|GetEagle_Spawn))
      (:%20%20
        (bind _output_get (Variables|Default|SetEagle_Spawn _result))
        (if (== _output_get 0)
          (CallFunction|SpawnEagle))))))

(event Input|AxisEvents|InputAxisMoveRight
  (params (AxisValue :type Float%20%28single-precision%29))
  ;[1 1 1] Chicken Movement
  (Variables|Default|SetGame_Start true)
  (if (Variables|Default|GetCan_Move)
    (if (!= AxisValue 0.0)
      (if (not (Variables|Default|GetInAir))
        (Character|LaunchCharacter (Math|Vector|MakeVector (* AxisValue -2e+02) 1.0 2e+02) true true)
        (Variables|Default|SetInAir true)
        (if (> AxisValue 0.0)
          (Transformation|SetActorRotation (Math|Rotator|MakeRotator 0.0 0.0 (Variables|Default|GetFaceRight)))
          (else
            (Transformation|SetActorRotation (Math|Rotator|MakeRotator 0.0 0.0 (Variables|Default|GetFaceLeft)))))
        (Audio|PlaySoundatLocation "/Game/Audio/hop_Cue.hop_Cue" (Transformation|GetActorLocation) "0, 0, 0" 1.0 1.0 0.0 0 0 0)
        (if (> (Math|Random|RandomFloat) 0.5)
          (Audio|PlaySoundatLocation "/Game/Audio/Bwak_Cue.Bwak_Cue" (Transformation|GetActorLocation) "0, 0, 0" 1.0 1.0 0.0 0 0 0))))))

(event Input|AxisEvents|InputAxisMoveForward
  (params (AxisValue :type Float%20%28single-precision%29))
  ;[1 1 1] Chicken Movement
  (Variables|Default|SetGame_Start true)
  (if (Variables|Default|GetCan_Move)
    (if (!= AxisValue 0.0)
      (if (not (Variables|Default|GetInAir))
        (Character|LaunchCharacter (Math|Vector|MakeVector 1.0 (* AxisValue 2e+02) 2e+02) true true)
        (Variables|Default|SetInAir true)
        (if (> AxisValue 0.0)
          (Transformation|SetActorRotation (Math|Rotator|MakeRotator 0.0 0.0 (Variables|Default|GetFaceForward)))
          (else
            (Transformation|SetActorRotation (Math|Rotator|MakeRotator 0.0 0.0 (Variables|Default|GetFaceBackward)))))
        (Audio|PlaySoundatLocation "/Game/Audio/hop_Cue.hop_Cue" (Transformation|GetActorLocation) "0, 0, 0" 1.0 1.0 0.0 0 0 0)
        (if (> (Math|Random|RandomFloat) 0.7)
          (Audio|PlaySoundatLocation "/Game/Audio/Bwak_Cue.Bwak_Cue" (Transformation|GetActorLocation) "0, 0, 0" 1.0 1.0 0.0 0 0 0))))))

(fn ConstructionScript)