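; BP_RailRoad is a railroad lane for a Crossy Road-style chicken game that periodically sends trains across at a random direction and speed.
; A frame-based Tick countdown spawns each BP_Train, with a Timeline flashing crossing lights and a warning sound playing shortly beforehand.
; Side kill zones destroy trains and reset the warning.
; Other triggers handle scoring, side blocking, eagle spawning and removing the lane with its trains.
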(event OnComponentBeginOverlap(LeftSideBlock)
  (params (OverlappedComponent :type Primitive%20Component%20Object%20Reference) (OtherActor :type Actor%20Object%20Reference) (OtherComp :type Primitive%20Component%20Object%20Reference) (OtherBodyIndex :type Integer) (bFromSweep :type Boolean) (SweepResult :type Hit%20Result%20Structure%20%28by%20ref%29))
  ;[1 1 1] Handle Chicken hitting world bounds
  (bind _asbp_my_character (Utilities|Casting|CastToBP_MyCharacter OtherActor))
  (Default|LeftBlock _asbp_my_character))

(event OnComponentBeginOverlap(RightSideBlock)
  (params (OverlappedComponent :type Primitive%20Component%20Object%20Reference) (OtherActor :type Actor%20Object%20Reference) (OtherComp :type Primitive%20Component%20Object%20Reference) (OtherBodyIndex :type Integer) (bFromSweep :type Boolean) (SweepResult :type Hit%20Result%20Structure%20%28by%20ref%29))
  ;[1 1 1] Handle Chicken hitting world bounds
  (bind _asbp_my_character (Utilities|Casting|CastToBP_MyCharacter OtherActor))
  (Default|RightBlock _asbp_my_character))

(event OnComponentBeginOverlap(Destroy_Right)
  (params (OverlappedComponent :type Primitive%20Component%20Object%20Reference) (OtherActor :type Actor%20Object%20Reference) (OtherComp :type Primitive%20Component%20Object%20Reference) (OtherBodyIndex :type Integer) (bFromSweep :type Boolean) (SweepResult :type Hit%20Result%20Structure%20%28by%20ref%29))
  (bind _light_intensity (Variables|Default|GetLight_Intensity))
  ;[1 1 1] Destroy the Vehicles as they cross the killzones
  (bind _asbp_train (Utilities|Casting|CastToBP_Train OtherActor))
  (Actor|DestroyActor _asbp_train)
  (Utilities|Array|RemoveItem (Variables|Default|GetTrain_Array) _asbp_train)
  (Rendering|Components|Light|SetIntensity (Variables|Default|GetRR_Light1) 0.0)
  ;[1 1 1] Handle Spawning the Vehicles in Lane and triggering RR Crossing
  (Rendering|Components|Light|SetIntensity (Variables|Default|GetRR_Light2) 0.0)
  (Variables|Default|SetSound%20Playing false)
  (bind (_direction _rr_light1_intensity _rr_light2_intensity) (Timeline|Timeline_0 Stop)
    (:Update
      (if (Variables|Default|GetSound%20Playing)
        _
        (else
          (Audio|PlaySoundatLocation "/Game/Audio/Train_Crossing_Cue.Train_Crossing_Cue" (Transformation|GetActorLocation) "0, 0, 0" 1.0 1.0 0.0 0 0 0)
          (Variables|Default|SetSound%20Playing true)))
      (Rendering|Components|Light|SetIntensity (Variables|Default|GetRR_Light1) (* _rr_light1_intensity _light_intensity))
      (Rendering|Components|Light|SetIntensity (Variables|Default|GetRR_Light2) (* _rr_light2_intensity _light_intensity))
      ;;[1 1 1] Decrement Spawn Time and Spawn Vehicle if equal to 0
      (Math|Integer|DecrementInt (Variables|Default|GetSpawn_Time)
        (:%20%20
          (if (== (Variables|Default|GetSpawn_Time) 0)
            (CallFunction|SpawnVehicle)
            (Variables|/Game/Blueprints/BP_Train.BP_Train_C|SetSet_Speed (Variables|Default|GetVehicle) (Variables|Default|GetLane_Speed))
            (Variables|Default|SetSpawn_Time (* (Math|Random|RandomIntegerinRange (Variables|Default|GetMin_Spawn_Time) (Variables|Default|GetMax_Spawn_Time)) 10))))))))

(event OnComponentBeginOverlap(LaneDestroyZone)
  (params (OverlappedComponent :type Primitive%20Component%20Object%20Reference) (OtherActor :type Actor%20Object%20Reference) (OtherComp :type Primitive%20Component%20Object%20Reference) (OtherBodyIndex :type Integer) (bFromSweep :type Boolean) (SweepResult :type Hit%20Result%20Structure%20%28by%20ref%29))
  (bind _train_array (Variables|Default|GetTrain_Array))
  ;[1 1 1] Handle destroying lanes
  (Utilities|Casting|CastToBP_MyCharacter OtherActor)
  (Actor|DestroyActor)
  ;[1 1 1] Hande destroying all BP_Train meshes within lane
  (for (_array_element _array_index) _train_array
    (Actor|DestroyActor _array_element)
    (Utilities|Array|SetArrayElem (Variables|Default|GetTrain_Array) _array_index 0))
  (Utilities|Array|Clear _train_array))

(event OnComponentBeginOverlap(Destroy_Left)
  (params (OverlappedComponent :type Primitive%20Component%20Object%20Reference) (OtherActor :type Actor%20Object%20Reference) (OtherComp :type Primitive%20Component%20Object%20Reference) (OtherBodyIndex :type Integer) (bFromSweep :type Boolean) (SweepResult :type Hit%20Result%20Structure%20%28by%20ref%29))
  (bind _light_intensity (Variables|Default|GetLight_Intensity))
  ;[1 1 1] Destroy the Vehicles as they cross the killzones
  (bind _asbp_train (Utilities|Casting|CastToBP_Train OtherActor))
  (Actor|DestroyActor _asbp_train)
  (Utilities|Array|RemoveItem (Variables|Default|GetTrain_Array) _asbp_train)
  (Rendering|Components|Light|SetIntensity (Variables|Default|GetRR_Light1) 0.0)
  ;[1 1 1] Handle Spawning the Vehicles in Lane and triggering RR Crossing
  (Rendering|Components|Light|SetIntensity (Variables|Default|GetRR_Light2) 0.0)
  (Variables|Default|SetSound%20Playing false)
  (bind (_direction _rr_light1_intensity _rr_light2_intensity) (Timeline|Timeline_0 Stop)
    (:Update
      (if (Variables|Default|GetSound%20Playing)
        _
        (else
          (Audio|PlaySoundatLocation "/Game/Audio/Train_Crossing_Cue.Train_Crossing_Cue" (Transformation|GetActorLocation) "0, 0, 0" 1.0 1.0 0.0 0 0 0)
          (Variables|Default|SetSound%20Playing true)))
      (Rendering|Components|Light|SetIntensity (Variables|Default|GetRR_Light1) (* _rr_light1_intensity _light_intensity))
      (Rendering|Components|Light|SetIntensity (Variables|Default|GetRR_Light2) (* _rr_light2_intensity _light_intensity))
      ;;[1 1 1] Decrement Spawn Time and Spawn Vehicle if equal to 0
      (Math|Integer|DecrementInt (Variables|Default|GetSpawn_Time)
        (:%20%20
          (if (== (Variables|Default|GetSpawn_Time) 0)
            (CallFunction|SpawnVehicle)
            (Variables|/Game/Blueprints/BP_Train.BP_Train_C|SetSet_Speed (Variables|Default|GetVehicle) (Variables|Default|GetLane_Speed))
            (Variables|Default|SetSpawn_Time (* (Math|Random|RandomIntegerinRange (Variables|Default|GetMin_Spawn_Time) (Variables|Default|GetMax_Spawn_Time)) 10))))))))

(event OnComponentHit(EagleKillZone)
  (params (HitComponent :type Primitive%20Component%20Object%20Reference) (OtherActor :type Actor%20Object%20Reference) (OtherComp :type Primitive%20Component%20Object%20Reference) (NormalImpulse :type Vector :default "0, 0, 0") (Hit :type Hit%20Result%20Structure%20%28by%20ref%29))
  (Utilities|FlowControl|DoOnce false
    (:Completed
      (bind _asbp_my_character (Utilities|Casting|CastToBP_MyCharacter OtherActor))
      (Default|SpawnEagle _asbp_my_character))))

(event OnComponentBeginOverlap(ScoringZone)
  (params (OverlappedComponent :type Primitive%20Component%20Object%20Reference) (OtherActor :type Actor%20Object%20Reference) (OtherComp :type Primitive%20Component%20Object%20Reference) (OtherBodyIndex :type Integer) (bFromSweep :type Boolean) (SweepResult :type Hit%20Result%20Structure%20%28by%20ref%29))
  (bind _asbp_my_character (Utilities|Casting|CastToBP_MyCharacter OtherActor))
  (Utilities|FlowControl|DoOnce false
    (:Completed
      (Default|UpdateScore _asbp_my_character))))

(event EventBeginPlay
  (bind _max_lane_speed (Variables|Default|GetMax_Lane_Speed))
  (bind _min_lane_speed (Variables|Default|GetMin_Lane_Speed))
  ;[1 1 1] Set Initial Spawning Variables of the Lane (Spawn Times, Vehicle Direction, and Vehicle Speed)
  (Variables|Default|SetDirection (Math|Random|RandomBool))
  (Variables|Default|SetSpawn_Time (* (Math|Random|RandomIntegerinRange (Variables|Default|GetMin_Spawn_Time) (Variables|Default|GetMax_Spawn_Time)) 10))
  (if (Variables|Default|GetDirection)
    (Variables|Default|SetLane_Speed (* (Math|Random|RandomFloatinRange _min_lane_speed _max_lane_speed) 1e+02))
    (else
      (Variables|Default|SetLane_Speed (* (Math|Random|RandomFloatinRange _min_lane_speed _max_lane_speed) -1e+02)))))

(event EventTick
  (params (DeltaSeconds :type Float%20%28single-precision%29))
  (bind _light_intensity (Variables|Default|GetLight_Intensity))
  ;[1 1 1] Handle Spawning the Vehicles in Lane and triggering RR Crossing
  (if (< (Variables|Default|GetSpawn_Time) 30)
    (bind (_direction _rr_light1_intensity _rr_light2_intensity) (Timeline|Timeline_0 Play)
      (:Update
        (if (Variables|Default|GetSound%20Playing)
          _
          (else
            (Audio|PlaySoundatLocation "/Game/Audio/Train_Crossing_Cue.Train_Crossing_Cue" (Transformation|GetActorLocation) "0, 0, 0" 1.0 1.0 0.0 0 0 0)
            (Variables|Default|SetSound%20Playing true)))
        (Rendering|Components|Light|SetIntensity (Variables|Default|GetRR_Light1) (* _rr_light1_intensity _light_intensity))
        (Rendering|Components|Light|SetIntensity (Variables|Default|GetRR_Light2) (* _rr_light2_intensity _light_intensity)))))
  ;;[1 1 1] Decrement Spawn Time and Spawn Vehicle if equal to 0
  (Math|Integer|DecrementInt (Variables|Default|GetSpawn_Time)
    (:%20%20
      (if (== (Variables|Default|GetSpawn_Time) 0)
        (CallFunction|SpawnVehicle)
        (Variables|/Game/Blueprints/BP_Train.BP_Train_C|SetSet_Speed (Variables|Default|GetVehicle) (Variables|Default|GetLane_Speed))
        (Variables|Default|SetSpawn_Time (* (Math|Random|RandomIntegerinRange (Variables|Default|GetMin_Spawn_Time) (Variables|Default|GetMax_Spawn_Time)) 10))))))

(fn ConstructionScript)

(fn SpawnVehicle
  ;[1 1 1] Spawn a Vehicle in Lane Based on Direction
  (if (Variables|Default|GetDirection)
    (bind _output_get (Variables|Default|SetStart (Transformation|GetWorldLocation (Variables|Default|GetLeft_Spawn))))
    (bind _returnvalue (Game|SpawnActorfromClass "/Game/Blueprints/BP_Train.BP_Train_C" (Math|Transform|MakeTransform _output_get "0, 0, 0" "1,1,1") "Undefined" 0 0))
    (bind _output_get_2 (Variables|Default|SetVehicle _returnvalue))
    (Utilities|Array|Add (Variables|Default|GetTrain_Array) _output_get_2)
    (else
      (bind _output_get_3 (Variables|Default|SetStart (Transformation|GetWorldLocation (Variables|Default|GetRight_Spawn))))
      (bind _returnvalue_2 (Game|SpawnActorfromClass "/Game/Blueprints/BP_Train.BP_Train_C" (Math|Transform|MakeTransform _output_get_3 "0.000000,180.000000, 0" "1,1,1") "Undefined" 0 0))
      (bind _output_get_4 (Variables|Default|SetVehicle _returnvalue_2))
      (Utilities|Array|Add (Variables|Default|GetTrain_Array) _output_get_4))))