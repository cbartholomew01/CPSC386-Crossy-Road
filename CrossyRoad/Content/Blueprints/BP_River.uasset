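; River lane in a Crossy Road-style game that the chicken crosses on logs or lily pads.
; BeginPlay picks the lane type, using the character's LilySpawned flag to prevent consecutive lily lanes, and randomizes log direction and speed.
; Tick either scatters static lily pads once or spawns random-sized logs on a countdown, both as BP_Log.
; Trigger zones clean up logs and the lane, and notify BP_MyCharacter of scoring, drowning, runoff and eagle attacks.
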(event OnComponentBeginOverlap(LeftSideBlock)
  (params (OverlappedComponent :type Primitive%20Component%20Object%20Reference) (OtherActor :type Actor%20Object%20Reference) (OtherComp :type Primitive%20Component%20Object%20Reference) (OtherBodyIndex :type Integer) (bFromSweep :type Boolean) (SweepResult :type Hit%20Result%20Structure%20%28by%20ref%29))
  ;[1 1 1] Handle when chicken gets too far to left or right of river
  (bind _asbp_my_character (Utilities|Casting|CastToBP_MyCharacter OtherActor))
  (Default|RiverRunoff _asbp_my_character))

(event OnComponentBeginOverlap(RightSideBlock)
  (params (OverlappedComponent :type Primitive%20Component%20Object%20Reference) (OtherActor :type Actor%20Object%20Reference) (OtherComp :type Primitive%20Component%20Object%20Reference) (OtherBodyIndex :type Integer) (bFromSweep :type Boolean) (SweepResult :type Hit%20Result%20Structure%20%28by%20ref%29))
  ;[1 1 1] Handle when chicken gets too far to left or right of river
  (bind _asbp_my_character (Utilities|Casting|CastToBP_MyCharacter OtherActor))
  (Default|RiverRunoff _asbp_my_character))

(event OnComponentHit(RiverKillZone)
  (params (HitComponent :type Primitive%20Component%20Object%20Reference) (OtherActor :type Actor%20Object%20Reference) (OtherComp :type Primitive%20Component%20Object%20Reference) (NormalImpulse :type Vector :default "0, 0, 0") (Hit :type Hit%20Result%20Structure%20%28by%20ref%29))
  (bind _asbp_my_character (Utilities|Casting|CastToBP_MyCharacter OtherActor))
  (Utilities|FlowControl|DoOnce false
    (:Completed
      (Default|FalleninRiver _asbp_my_character))))

(event OnComponentBeginOverlap(LaneDestroyZone)
  (params (OverlappedComponent :type Primitive%20Component%20Object%20Reference) (OtherActor :type Actor%20Object%20Reference) (OtherComp :type Primitive%20Component%20Object%20Reference) (OtherBodyIndex :type Integer) (bFromSweep :type Boolean) (SweepResult :type Hit%20Result%20Structure%20%28by%20ref%29))
  (bind _log_array (Variables|Default|GetLog_Array))
  ;[1 1 1] Handle destroying lanes
  (Utilities|Casting|CastToBP_MyCharacter OtherActor)
  (Actor|DestroyActor)
  ;[1 1 1] Hande destroying all BP_Log meshes within lane
  (for (_array_element _array_index) _log_array
    (Actor|DestroyActor _array_element)
    (Utilities|Array|SetArrayElem (Variables|Default|GetLog_Array) _array_index 0))
  (Utilities|Array|Clear _log_array))

(event OnComponentBeginOverlap(Destroy_Left)
  (params (OverlappedComponent :type Primitive%20Component%20Object%20Reference) (OtherActor :type Actor%20Object%20Reference) (OtherComp :type Primitive%20Component%20Object%20Reference) (OtherBodyIndex :type Integer) (bFromSweep :type Boolean) (SweepResult :type Hit%20Result%20Structure%20%28by%20ref%29))
  ;[1 1 1] Destroy the Vehicles as they cross the killzones
  (bind _asbp_log (Utilities|Casting|CastToBP_Log OtherActor))
  (Actor|DestroyActor _asbp_log)
  ;[1 1 1] Remove instances of destroyed BP_Log from array
  (Utilities|Array|RemoveItem (Variables|Default|GetLog_Array) _asbp_log))

(event OnComponentHit(EagleKillZone)
  (params (HitComponent :type Primitive%20Component%20Object%20Reference) (OtherActor :type Actor%20Object%20Reference) (OtherComp :type Primitive%20Component%20Object%20Reference) (NormalImpulse :type Vector :default "0, 0, 0") (Hit :type Hit%20Result%20Structure%20%28by%20ref%29))
  (Utilities|FlowControl|DoOnce false
    (:Completed
      (bind _asbp_my_character (Utilities|Casting|CastToBP_MyCharacter OtherActor))
      (Default|SpawnEagle _asbp_my_character))))

(event OnComponentBeginOverlap(Destroy_Right)
  (params (OverlappedComponent :type Primitive%20Component%20Object%20Reference) (OtherActor :type Actor%20Object%20Reference) (OtherComp :type Primitive%20Component%20Object%20Reference) (OtherBodyIndex :type Integer) (bFromSweep :type Boolean) (SweepResult :type Hit%20Result%20Structure%20%28by%20ref%29))
  ;[1 1 1] Destroy the Vehicles as they cross the killzones
  (bind _asbp_log (Utilities|Casting|CastToBP_Log OtherActor))
  (Actor|DestroyActor _asbp_log)
  ;[1 1 1] Remove instances of destroyed BP_Log from array
  (Utilities|Array|RemoveItem (Variables|Default|GetLog_Array) _asbp_log))

(event OnComponentBeginOverlap(ScoringZone)
  (params (OverlappedComponent :type Primitive%20Component%20Object%20Reference) (OtherActor :type Actor%20Object%20Reference) (OtherComp :type Primitive%20Component%20Object%20Reference) (OtherBodyIndex :type Integer) (bFromSweep :type Boolean) (SweepResult :type Hit%20Result%20Structure%20%28by%20ref%29))
  (bind _asbp_my_character (Utilities|Casting|CastToBP_MyCharacter OtherActor))
  (Utilities|FlowControl|DoOnce false
    (:Completed
      (Default|UpdateScore _asbp_my_character))))

(event EventBeginPlay
  (bind _max_lane_speed (Variables|Default|GetMax_Lane_Speed))
  (bind _min_lane_speed (Variables|Default|GetMin_Lane_Speed))
  (bind _asbp_my_character (Utilities|Casting|CastToBP_MyCharacter (Game|GetPlayerCharacter 0)))
  (if (Variables|/Game/Blueprints/BP_MyCharacter.BP_MyCharacter_C|GetLily_Spawned _asbp_my_character)
    (Variables|/Game/Blueprints/BP_MyCharacter.BP_MyCharacter_C|SetLily_Spawned _asbp_my_character false :!label _label)
    ;[1 1 1] Set Initial Spawning Variables of the Lane (Spawn Times, Vehicle Direction, and Vehicle Speed)
    (Variables|Default|SetDirection (Math|Random|RandomBool))
    (Variables|Default|SetSpawn_Time (* (Math|Random|RandomIntegerinRange (Variables|Default|GetMin_Spawn_Time) (Variables|Default|GetMax_Spawn_Time)) 10))
    (if (Variables|Default|GetDirection)
      (Variables|Default|SetLane_Speed (* (Math|Random|RandomFloatinRange _min_lane_speed _max_lane_speed) 5e+01))
      (else
        (Variables|Default|SetLane_Speed (* (Math|Random|RandomFloatinRange _min_lane_speed _max_lane_speed) -5e+01))))
    (elif (> (Math|Random|RandomFloat) 0.4)
      (Variables|Default|SetLilly_Lane true)
      (Variables|/Game/Blueprints/BP_MyCharacter.BP_MyCharacter_C|SetLily_Spawned _asbp_my_character true)
      (else
        (goto _label)))))

(event EventTick
  (params (DeltaSeconds :type Float%20%28single-precision%29))
  (if (Variables|Default|GetLilly_Lane)
    (Utilities|FlowControl|DoOnce false
      (:Completed
        (Variables|Default|SetRandom_Start (Transformation|GetWorldLocation (Variables|Default|GetRandomStart)))
        (Variables|Default|SetRandom_End (Transformation|GetWorldLocation (Variables|Default|GetRandomEnd)))
        (for _index (range 0 (Math|Float|Truncate (/ (Math|Vector|Distance(Vector) (Variables|Default|GetRandom_Start) (Variables|Default|GetRandom_End)) 8e+01)))
          (if (> (Math|Random|RandomFloat) 0.5)
            (if (> (Math|Random|RandomFloat) 0.5)
              (CallFunction|SpawnObstacle (Math|Vector|MakeVector (.x (+ (Math|Vector|MakeVector (.x (Variables|Default|GetRandom_Start)) 0.0 0.0) (* _index 80))) (.y (Variables|Default|GetRandom_Start)) (.z (Variables|Default|GetRandom_Start))))
              (Utilities|FlowControl|DoOnce false
                (:Completed
                  (Audio|PlaySoundatLocation "/Game/Audio/River_Cue.River_Cue" (Transformation|GetActorLocation) "0, 0, 0" 1.0 1.0 0.0 0 0 0))))))))
    (else
      ;[1 1 1] Handle Spawning the Vehicles in Lane
      ;;[1 1 1] Decrement Spawn Time and Spawn Vehicle if equal to 0
      (Math|Integer|DecrementInt (Variables|Default|GetSpawn_Time)
        (:%20%20
          (if (== (Variables|Default|GetSpawn_Time) 0)
            (CallFunction|SpawnVehicle)
            (Variables|/Game/Blueprints/BP_Log.BP_Log_C|SetSet_Speed (Variables|Default|GetVehicle) (Variables|Default|GetLane_Speed))
            (Variables|Default|SetSpawn_Time (* (Math|Random|RandomIntegerinRange (Variables|Default|GetMin_Spawn_Time) (Variables|Default|GetMax_Spawn_Time)) 10))
            (Components|StaticMesh|SetStaticMesh (Variables|/Game/Blueprints/BP_Log.BP_Log_C|GetStaticMesh (Variables|Default|GetVehicle)) (Utilities|Select :Index (Math|Random|RandomIntegerinRange 0 2) :Option%200 "/Game/Meshes/LogS.LogS" :Option%201 "/Game/Meshes/LogM.LogM" :Option%202 "/Game/Meshes/LogL.LogL"))
            (Utilities|FlowControl|DoOnce false
              (:Completed
                (Audio|PlaySoundatLocation "/Game/Audio/River_Cue.River_Cue" (Transformation|GetActorLocation) "0, 0, 0" 1.0 1.0 0.0 0 0 0)))))))))

(fn ConstructionScript)

(fn SpawnVehicle
  ;[1 1 1] Spawn a Vehicle in Lane Based on Direction
  (if (Variables|Default|GetDirection)
    (bind _output_get (Variables|Default|SetStart (Transformation|GetWorldLocation (Variables|Default|GetLeft_Spawn))))
    (bind _returnvalue (Game|SpawnActorfromClass "/Game/Blueprints/BP_Log.BP_Log_C" (Math|Transform|MakeTransform _output_get "0, 0, 0" "1,1,1") "Undefined" 0 0))
    (bind _output_get_2 (Variables|Default|SetVehicle _returnvalue))
    (Utilities|Array|Add (Variables|Default|GetLog_Array) _output_get_2)
    (else
      (bind _output_get_3 (Variables|Default|SetStart (Transformation|GetWorldLocation (Variables|Default|GetRight_Spawn))))
      (bind _returnvalue_2 (Game|SpawnActorfromClass "/Game/Blueprints/BP_Log.BP_Log_C" (Math|Transform|MakeTransform _output_get_3 "0.000000,180.000000, 0" "1,1,1") "Undefined" 0 0))
      (bind _output_get_4 (Variables|Default|SetVehicle _returnvalue_2))
      (Utilities|Array|Add (Variables|Default|GetLog_Array) _output_get_4))))

(fn SpawnObstacle
  (params (Location :type Vector))
  ;[1 1 1] Spawn a Vehicle in Lane Based on Direction
  (bind _returnvalue (Game|SpawnActorfromClass "/Game/Blueprints/BP_Log.BP_Log_C" (Math|Transform|MakeTransform Location "0, 0, 0" "1,1,1") "Undefined" 0 0))
  (bind _output_get (Variables|Default|SetVehicle _returnvalue))
  (Components|StaticMesh|SetStaticMesh (Variables|/Game/Blueprints/BP_Log.BP_Log_C|GetStaticMesh _output_get) "/Game/Meshes/Obstacles/lilypad.lilypad")
  (Utilities|Array|Add (Variables|Default|GetLog_Array) _output_get))