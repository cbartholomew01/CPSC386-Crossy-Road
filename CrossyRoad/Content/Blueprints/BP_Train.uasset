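; BP_Train is a moving train hazard that ends the run of the chicken player character (BP_MyCharacter) on contact.
; Tick slides it along world X at SetSpeed, scaled by delta time, with sweep enabled.
; Overlapping KillZone calls RunOver on the character, while overlapping any of three static meshes calls JumpedIntoCar.
; Each overlap handler has its own DoOnce, so it fires once per train instance.
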(event OnComponentBeginOverlap(KillZone)
  (params (OverlappedComponent :type Primitive%20Component%20Object%20Reference) (OtherActor :type Actor%20Object%20Reference) (OtherComp :type Primitive%20Component%20Object%20Reference) (OtherBodyIndex :type Integer) (bFromSweep :type Boolean) (SweepResult :type Hit%20Result%20Structure%20%28by%20ref%29))
  ;[1 1 1] Chicken Collision on X and Y Plane
  (bind _asbp_my_character (Utilities|Casting|CastToBP_MyCharacter OtherActor))
  (Utilities|FlowControl|DoOnce false
    (:Completed
      (Default|RunOver _asbp_my_character))))

(event OnComponentBeginOverlap(StaticMesh)
  (params (OverlappedComponent :type Primitive%20Component%20Object%20Reference) (OtherActor :type Actor%20Object%20Reference) (OtherComp :type Primitive%20Component%20Object%20Reference) (OtherBodyIndex :type Integer) (bFromSweep :type Boolean) (SweepResult :type Hit%20Result%20Structure%20%28by%20ref%29))
  ;[1 1 1] Chicken Collision on X and Y Plane
  (bind _asbp_my_character (Utilities|Casting|CastToBP_MyCharacter OtherActor))
  (Utilities|FlowControl|DoOnce false
    (:Completed
      (Default|JumpedIntoCar _asbp_my_character))))

(event OnComponentBeginOverlap(StaticMesh1)
  (params (OverlappedComponent :type Primitive%20Component%20Object%20Reference) (OtherActor :type Actor%20Object%20Reference) (OtherComp :type Primitive%20Component%20Object%20Reference) (OtherBodyIndex :type Integer) (bFromSweep :type Boolean) (SweepResult :type Hit%20Result%20Structure%20%28by%20ref%29))
  ;[1 1 1] Chicken Collision on X and Y Plane
  (bind _asbp_my_character (Utilities|Casting|CastToBP_MyCharacter OtherActor))
  (Utilities|FlowControl|DoOnce false
    (:Completed
      (Default|JumpedIntoCar _asbp_my_character))))

(event OnComponentBeginOverlap(StaticMesh2)
  (params (OverlappedComponent :type Primitive%20Component%20Object%20Reference) (OtherActor :type Actor%20Object%20Reference) (OtherComp :type Primitive%20Component%20Object%20Reference) (OtherBodyIndex :type Integer) (bFromSweep :type Boolean) (SweepResult :type Hit%20Result%20Structure%20%28by%20ref%29))
  ;[1 1 1] Chicken Collision on X and Y Plane
  (bind _asbp_my_character (Utilities|Casting|CastToBP_MyCharacter OtherActor))
  (Utilities|FlowControl|DoOnce false
    (:Completed
      (Default|JumpedIntoCar _asbp_my_character))))

(event EventTick
  (params (DeltaSeconds :type Float%20%28single-precision%29))
  ;[1 1 1] Train Movement
  (Transformation|AddActorWorldOffset (Math|Vector|MakeVector (* DeltaSeconds (Variables|Default|GetSet_Speed)) 0.0 0.0) true))

(fn ConstructionScript)